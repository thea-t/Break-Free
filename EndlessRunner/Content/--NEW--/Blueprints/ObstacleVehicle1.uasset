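; ObstacleVehicle1 is a moving obstacle vehicle, built around a SWAT van component, that travels along the world X axis.
; Tick offsets the actor by MovementSpeed scaled by delta time, without sweeping for collisions.
; OnSpeedIncrease subtracts its argument from MovementSpeed, so speeding up implies travel toward negative X.
; BeginPlay caches the van component's relative location, which OnReset applies as the actor's relative location.
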(event EventTick
  (params (DeltaSeconds :type Float%20%28single-precision%29))
  (Transformation|SetActorLocation (+ (Transformation|GetActorLocation) (Math|Vector|MakeVector (* DeltaSeconds (Variables|Default|GetmovementSpeed)) 0.0 0.0)) false false))

(event EventBeginPlay
  (Variables|Default|SetstartPos (.Location (Math|Transform|BreakTransform (Transformation|GetRelativeTransform (Variables|Default|Getvan_SWAT_van_SWAT))))))

(fn ConstructionScript)

(fn OnReset
  (Transformation|SetActorRelativeLocation (Variables|Default|GetstartPos)))

(fn OnSpeedIncrease
  (params (speedIncreasePerSecond :type Float%20%28single-precision%29))
  (Variables|Default|SetmovementSpeed (- (Variables|Default|GetmovementSpeed) speedIncreasePerSecond)))