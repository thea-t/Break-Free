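; ObstacleVehicle is a vehicle obstacle that drives in a straight line along the world X axis.
; It records its start location on BeginPlay, then offsets its position every Tick by MovementSpeed scaled by delta time, teleporting without sweep.
; OnReset moves it back to that start location, also without sweep.
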(event EventTick
  (params (DeltaSeconds :type Float%20%28single-precision%29))
  (Transformation|SetActorLocation (+ (Transformation|GetActorLocation) (Math|Vector|MakeVector (* DeltaSeconds (Variables|Default|GetmovementSpeed)) 0.0 0.0)) false true))

(event EventBeginPlay
  (Variables|Default|SetstartPos (Transformation|GetActorLocation)))

(fn ConstructionScript)

(fn OnReset
  (Transformation|SetActorLocation (Variables|Default|GetstartPos) false false))