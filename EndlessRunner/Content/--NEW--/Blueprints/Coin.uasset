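; Coin pickup actor that spins in the world and can be collected by the player.
; Tick calls AnimateCoin, which applies a fixed per-frame rotation, so spin speed varies with frame rate.
; Overlap by an actor tagged Player that casts to ThirdPersonCharacter calls OnCoinCollected on it.
; SetActive then hides the mesh and collider and disables collision instead of destroying the coin.
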(event OnComponentBeginOverlap(Collider)
  (params (OverlappedComponent :type Primitive%20Component%20Object%20Reference) (OtherActor :type Actor%20Object%20Reference) (OtherComp :type Primitive%20Component%20Object%20Reference) (OtherBodyIndex :type Integer) (bFromSweep :type Boolean) (SweepResult :type Hit%20Result%20Structure%20%28by%20ref%29))
  (if (Actor|ActorHasTag OtherActor "Player")
    (bind _asthird_person_character (Utilities|Casting|CastToThirdPersonCharacter OtherActor))
    (Default|OnCoinCollected _asthird_person_character)
    (CallFunction|SetActive false)))

(event EventTick
  (params (DeltaSeconds :type Float%20%28single-precision%29))
  (CallFunction|AnimateCoin 0.0))

(fn ConstructionScript)

(fn AnimateCoin
  (params (deltaTime :type Float%20%28single-precision%29))
  (Class|Actor|AddActorWorldRotation "0,5.000000, 0"))

(fn SetActive
  (params (active :type Boolean))
  (Rendering|SetVisibility (Variables|Default|GetStaticMesh) active false)
  (Rendering|SetVisibility (Variables|Default|GetCollider) active false)
  (if active
    (Collision|SetCollisionEnabled (Variables|Default|GetCollider) "QueryOnly")
    (else
      (Collision|SetCollisionEnabled (Variables|Default|GetCollider) "NoCollision"))))