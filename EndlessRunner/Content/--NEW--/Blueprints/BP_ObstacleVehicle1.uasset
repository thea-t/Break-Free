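; BP_ObstacleVehicle1 is a moving SWAT van obstacle that travels along the world X axis every frame at MovementSpeed, scaled by delta time, without sweeping.
; BeginPlay saves the van component's relative location, and OnReset applies that saved value as the actor's relative location.
; OnSpeedIncrease subtracts the given increment from MovementSpeed, pushing the velocity further toward negative X.
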(event EventTick
  (params (DeltaSeconds :type Float%20%28single-precision%29))
  ;[1 1 1] Moving the vehicle
  (Transformation|SetActorLocation (+ (Transformation|GetActorLocation) (Math|Vector|MakeVector (* DeltaSeconds (Variables|Default|GetmovementSpeed)) 0.0 0.0)) false false))

(event EventBeginPlay
  ;[1 1 1] Save the vehicle's starting pos
  (Variables|Default|SetstartPos (.Location (Math|Transform|BreakTransform (Transformation|GetRelativeTransform (Variables|Default|Getvan_SWAT_van_SWAT))))))

(fn ConstructionScript)

(fn OnReset
  (Transformation|SetActorRelativeLocation (Variables|Default|GetstartPos)))

(fn OnSpeedIncrease
  (params (speedIncreasePerSecond :type Float%20%28single-precision%29))
  ;[1 1 1] Chanigng the movement speed
  (Variables|Default|SetmovementSpeed (- (Variables|Default|GetmovementSpeed) speedIncreasePerSecond)))