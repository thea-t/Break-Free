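; ChunkManager scrolls level chunks along the X axis and recycles them to form an endless track.
; Each Tick it teleports every upcoming chunk by MovementSpeed, and any crossing a fixed negative X threshold moves into a passed pool.
; A random chunk from that pool, possibly the same one, is then repositioned at the end of the line by ChunkLength and has its ChunkBase coins reactivated.
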(event EventTick
  (params (DeltaSeconds :type Float%20%28single-precision%29))
  (CallFunction|MoveUpcomingChunks DeltaSeconds))

(fn ConstructionScript)

(fn MoveUpcomingChunks
  (params (deltaTime :type Float%20%28single-precision%29))
  (for _array_element (Variables|Default|GetUpcomingChunks)
    (Transformation|SetActorLocation _array_element (+ (Transformation|GetActorLocation _array_element) (Math|Vector|MakeVector (* deltaTime (Variables|Default|GetmovementSpeed)) 0.0 0.0)) false true)
    (Math|Float|CompareFloat (.X (Math|Vector|BreakVector (+ (Transformation|GetActorLocation _array_element) (Math|Vector|MakeVector (* deltaTime (Variables|Default|GetmovementSpeed)) 0.0 0.0)))) -6e+03
      (:<
        (CallFunction|OnChunkPassed _array_element)))))

(fn OnChunkPassed
  (params (passedChunk :type Actor%20Object%20Reference))
  (bind _output_get (Variables|Default|SetpassedChunk passedChunk))
  (Utilities|Array|Add (Variables|Default|GetPassedChunks) _output_get)
  (Utilities|Array|RemoveItem (Variables|Default|GetUpcomingChunks) passedChunk)
  (bind _output_get_2 (Variables|Default|SetnextChunk (.OutItem (Utilities|Array|Random (Variables|Default|GetPassedChunks)))))
  (Transformation|SetActorLocation _output_get_2 (Math|Vector|MakeVector (* (- (Utilities|Array|Length (Variables|Default|GetUpcomingChunks)) 1) (Variables|Default|GetchunkLength)) 0.0 0.0) false false)
  (Utilities|Array|Add (Variables|Default|GetUpcomingChunks) (Variables|Default|GetnextChunk))
  (Utilities|Array|RemoveItem (Variables|Default|GetPassedChunks) (Variables|Default|GetnextChunk))
  (CallFunction|ResetChunk (Variables|Default|GetnextChunk)))

(fn ResetChunk
  (params (chunkToReset :type Actor%20Object%20Reference))
  (bind _aschunk_base (Utilities|Casting|CastToChunkBase chunkToReset))
  (for _array_element (Variables|/Game/--NEW--/Blueprints/ChunkBase.ChunkBase_C|GetcoinsArray _aschunk_base)
    (Default|SetActive _array_element true)))