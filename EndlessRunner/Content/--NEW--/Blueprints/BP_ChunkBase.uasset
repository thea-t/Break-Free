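; BP_ChunkBase is a base level-chunk actor that tracks the coins and obstacle vehicles placed inside it as child actors.
; On BeginPlay it sorts all child actors by Coin, SWATVehicle and PoliceVehicle tags, casting each into its own typed array.
; OnSpeedIncrease relays speed changes to both vehicle arrays, passing SpeedPerSecond to SWAT vehicles but a fixed zero to police vehicles.
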(event EventBeginPlay
  ;[1 1 1] Add all the coins and vehicles to their arrays
  (for _array_element (Actor|GetAllChildActors true)
    (if (Actor|ActorHasTag _array_element "Coin")
      (bind _asbp_coin (Utilities|Casting|CastToBP_Coin _array_element))
      (Utilities|Array|Add (Variables|Default|GetcoinsArray) _asbp_coin)
      (elif (Actor|ActorHasTag _array_element "SWATVehicle")
        (bind _asbp_obstacle_vehicle (Utilities|Casting|CastToBP_ObstacleVehicle _array_element))
        (Utilities|Array|Add (Variables|Default|GetswatVehicleObstaclesArray) _asbp_obstacle_vehicle)
        (elif (Actor|ActorHasTag _array_element "PoliceVehicle")
          (bind _asbp_obstacle_vehicle_1 (Utilities|Casting|CastToBP_ObstacleVehicle1 _array_element))
          (Utilities|Array|Add (Variables|Default|GetpoliceVehicleObstaclesArray) _asbp_obstacle_vehicle_1))))))

(fn ConstructionScript)

(fn OnSpeedIncrease
  (params (speedPerSecond :type Float%20%28single-precision%29))
  ;[1 1 1] Increase speed of the vehicles
  (for _array_element (Variables|Default|GetswatVehicleObstaclesArray)
    (Default|OnSpeedIncrease _array_element speedPerSecond))
  (for _array_element_2 (Variables|Default|GetpoliceVehicleObstaclesArray)
    (Default|OnSpeedIncrease _array_element_2 0.0)))