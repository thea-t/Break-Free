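; ChunkBase is a Blueprint base for level chunks that contain coins and vehicle obstacles as child actors.
; On BeginPlay it scans its child actors by tag, storing Coin-tagged ones in a coin array and Vehicle-tagged ones in an obstacle vehicle array.
; OnSpeedIncrease forwards a speed-per-second value to every stored vehicle obstacle; the coin array is only populated here.
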(event EventBeginPlay
  (for _array_element (Actor|GetAllChildActors true)
    (if (Actor|ActorHasTag _array_element "Coin")
      (bind _ascoin (Utilities|Casting|CastToCoin _array_element))
      (Utilities|Array|Add (Variables|Default|GetcoinsArray) _ascoin)
      (elif (Actor|ActorHasTag _array_element "Vehicle")
        (bind _asobstacle_vehicle (Utilities|Casting|CastToObstacleVehicle _array_element))
        (Utilities|Array|Add (Variables|Default|GetvehicleObstaclesArray) _asobstacle_vehicle)))))

(fn ConstructionScript)

(fn OnSpeedIncrease
  (params (speedPerSecond :type Float%20%28single-precision%29))
  (for _array_element (Variables|Default|GetvehicleObstaclesArray)
    (Default|OnSpeedIncrease _array_element speedPerSecond)))