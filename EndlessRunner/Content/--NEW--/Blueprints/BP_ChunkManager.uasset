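; Chunk manager for an endless runner that scrolls level chunks along X past the player until the player dies.
; Tick moves upcoming chunks and, about every second, raises the scroll speed and notifies all chunks.
; Chunks are pooled: one passing the rear threshold joins the passed pool, then a random pooled chunk moves to the track's end.
; The recycled chunk gets its coins and SWAT vehicle obstacles reset.
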(event Custom|OnSpeedIncrease
  ;[1 1 1] Increasing the speed of all the chunks
  (Variables|Default|SetpassedTime 0.0)
  (Variables|Default|SetmovementSpeed (- (Variables|Default|GetmovementSpeed) (Variables|Default|GetspeedIncreaseEverySecond)))
  (for _array_element (Variables|Default|GetUpcomingChunks)
    (bind _asbp_chunk_base (Utilities|Casting|CastToBP_ChunkBase _array_element))
    (Default|OnSpeedIncrease _asbp_chunk_base (Variables|Default|GetspeedIncreaseEverySecond)))
  (for _array_element_2 (Variables|Default|GetPassedChunks)
    (bind _asbp_chunk_base_2 (Utilities|Casting|CastToBP_ChunkBase _array_element_2))
    (Default|OnSpeedIncrease _asbp_chunk_base_2 (Variables|Default|GetspeedIncreaseEverySecond))))

(event EventTick
  (params (DeltaSeconds :type Float%20%28single-precision%29))
  ;[1 1 1] Move Chunks
  (if (not (Variables|/Game/ThirdPersonBP/Blueprints/BP_ThirdPersonCharacter.BP_ThirdPersonCharacter_C|GetisDead (Variables|Default|Getplayer)))
    (CallFunction|MoveUpcomingChunks DeltaSeconds)
    (bind _output_get (Variables|Default|SetpassedTime (+ DeltaSeconds (Variables|Default|GetpassedTime))))
    (Math|Float|CompareFloat _output_get 1.0
      (:>
        (CallFunction|OnSpeedIncrease)))))

(fn ConstructionScript)

(fn MoveUpcomingChunks
  (params (deltaTime :type Float%20%28single-precision%29))
  ;[1 1 1] Moving each upcoming chunk and check when a chunk had passed the player
  (for _array_element (Variables|Default|GetUpcomingChunks)
    (Transformation|SetActorLocation _array_element (+ (Transformation|GetActorLocation _array_element) (Math|Vector|MakeVector (* deltaTime (Variables|Default|GetmovementSpeed)) 0.0 0.0)) false true)
    (Math|Float|CompareFloat (.X (Math|Vector|BreakVector (+ (Transformation|GetActorLocation _array_element) (Math|Vector|MakeVector (* deltaTime (Variables|Default|GetmovementSpeed)) 0.0 0.0)))) -6e+03
      (:<
        (CallFunction|OnChunkPassed _array_element)))))

(fn OnChunkPassed
  (params (passedChunk :type Actor%20Object%20Reference))
  ;[1 1 1] Object Pulling with the chunks
  (bind _output_get (Variables|Default|SetpassedChunk passedChunk))
  (Utilities|Array|Add (Variables|Default|GetPassedChunks) _output_get)
  (Utilities|Array|RemoveItem (Variables|Default|GetUpcomingChunks) passedChunk)
  (bind _output_get_2 (Variables|Default|SetnextChunk (.OutItem (Utilities|Array|Random (Variables|Default|GetPassedChunks)))))
  (Transformation|SetActorLocation _output_get_2 (Math|Vector|MakeVector (* (- (Utilities|Array|Length (Variables|Default|GetUpcomingChunks)) 1) (Variables|Default|GetchunkLength)) 0.0 0.0) false false)
  (Utilities|Array|Add (Variables|Default|GetUpcomingChunks) (Variables|Default|GetnextChunk))
  (Utilities|Array|RemoveItem (Variables|Default|GetPassedChunks) (Variables|Default|GetnextChunk))
  (CallFunction|ResetChunk (Variables|Default|GetnextChunk)))

(fn ResetChunk
  (params (chunkToReset :type Actor%20Object%20Reference))
  ;[1 1 1] Resetting each coin and vehicle
  (bind _asbp_chunk_base (Utilities|Casting|CastToBP_ChunkBase chunkToReset))
  (for _array_element (Variables|/Game/--NEW--/Blueprints/BP_ChunkBase.BP_ChunkBase_C|GetcoinsArray _asbp_chunk_base)
    (Default|SetActive _array_element true))
  (for _array_element_2 (Variables|/Game/--NEW--/Blueprints/BP_ChunkBase.BP_ChunkBase_C|GetswatVehicleObstaclesArray _asbp_chunk_base)
    (Default|OnReset _array_element_2)))